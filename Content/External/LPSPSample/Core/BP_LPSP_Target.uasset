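; Shooting target actor for the LPSP sample that reacts to point and radial damage through interface events.
; Point damage runs a collapsed graph that, while active, plays an animation and sound, deactivates, then reactivates with another animation and sound after a random delay.
; Radial damage spawns an actor at the mesh transform and destroys the target.
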(event `self.On Receive Damage Point`
  ;[1 0.03719 0] Point Damage
  (if (`self.Active`)
    (`GameplayStatics.SpawnSoundAtLocation` null (`SceneComponent.K2_GetComponentLocation` (`self.Mesh`)) (struct) 1.0 1.0 0.0 null null)
    (`SkeletalMeshComponent.PlayAnimation` (`self.Mesh`) null false)
    (set `self.Active` false)
    (`KismetSystemLibrary.Delay` (`KismetMathLibrary.RandomFloatInRange` 1.0 10.0))
    (set `self.Active` true)
    (`SkeletalMeshComponent.PlayAnimation` (`self.Mesh`) null false)
    (`GameplayStatics.SpawnSoundAtLocation` null (`SceneComponent.K2_GetComponentLocation` (`self.Mesh`)) (struct) 1.0 1.0 0.0 null null)))

(event `self.On Receive Damage Radial`
  ;[1 0.1603 0] Radial Damage
  (`|SpawnActorFromClass` null (`SceneComponent.K2_GetComponentToWorld` (`self.Mesh`)) "AlwaysSpawn" "OverrideRootScale" null null)
  (`self.K2_DestroyActor`))

(fn `UserConstructionScript`)