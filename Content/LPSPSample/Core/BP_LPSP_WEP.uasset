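; Base weapon Blueprint for the LPSP sample, handling hitscan firing, reloading and ammunition, with getters for weapon stats and HUD textures.
; Firing plays a montage, decrements ammo, spawns a muzzle flash and traces from the muzzle toward a point along the camera's forward vector.
; Hits spawn decal, particles and sound, then message damage to the actor.
; Reload picks the empty or regular montage and refills ammo on blend-out.
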(event `self.ReceiveBeginPlay`
  ;[1 1 1] Begin Play
  (`parent.ReceiveBeginPlay`)
  (set `self.AmmunitionCurrent` (`self.AmmunitionMax`)))

(event `self.On Reload`
  ;[0.6172 1 0] Reload
  (bind _returnvalue (`self.Is Empty`))
  (bind _returnvalue_2 (select `bool` _returnvalue :`false` (`self.MontageReload`) :`true` (`self.MontageReloadEmpty`)))
  (`/Engine/EditorBlueprintResources/StandardMacros.IsValid` _returnvalue_2
    (:`Is Valid`
      (`|PlayMontage` (`self.Mesh Weapon`) _returnvalue_2
        (:`OnBlendOut`
          (set `self.AmmunitionCurrent` (`self.AmmunitionMax`)))))))

(event `self.On Fire`
  (bind _returnvalue (`GameplayStatics.GetPlayerCameraManager` 0))
  (bind (_bblockinghit _binitialoverlap _time _distance _location _impactpoint _normal _impactnormal) (`GameplayStatics.BreakHitResult` (`self.HitResult`)))
  (bind (_bblockinghit_2 _binitialoverlap_2 _time_2 _distance_2 _location_2 _impactpoint_2 _normal_2 _impactnormal_2) (`GameplayStatics.BreakHitResult` (`self.HitResult`)))
  ;[0.125 0 1] Fire
  (`/Engine/EditorBlueprintResources/StandardMacros.IsValid` (`self.MontageFire`)
    (:`Is Valid`
      (`|PlayMontage` (`self.Mesh Weapon`) (`self.MontageFire`)
        (:`then`
          (set `self.AmmunitionCurrent` (`KismetMathLibrary.Clamp` (- (`self.AmmunitionCurrent`) 1) 0 (`self.AmmunitionMax`)))
          (`GameplayStatics.SpawnEmitterAttached` "/LPSPSample/LPSPSample/Art/Effects/PS_MFlash.PS_MFlash" (`self.Mesh Weapon`) "SOCKET_Muzzle" (0.0 0.0 0.0) (struct :`Yaw` 90.0))
          (bind (_outhit _returnvalue_2) (`KismetSystemLibrary.LineTraceSingle` (.location (`SceneComponent.GetSocketTransform` (`self.Mesh Weapon`) "SOCKET_Muzzle" "RTS_World")) (+ (`PlayerCameraManager.GetCameraLocation` _returnvalue) (* (`KismetMathLibrary.GetForwardVector` (`PlayerCameraManager.GetCameraRotation` _returnvalue)) 10000.0)) "TraceTypeQuery1"))
          (set `self.HitResult` _outhit)
          (if _returnvalue_2
            (`GameplayStatics.SpawnDecalAtLocation` "/LPSPSample/LPSPSample/Art/Effects/MI_Decal_Bullet_Concrete.MI_Decal_Bullet_Concrete" (5.0 5.0 5.0) _impactpoint (`KismetMathLibrary.Conv_VectorToRotator` _impactnormal) 15.0)
            (`GameplayStatics.SpawnEmitterAtLocation` "/LPSPSample/LPSPSample/Art/Effects/PS_Impact.PS_Impact" _impactpoint_2 (`KismetMathLibrary.Conv_VectorToRotator` _impactnormal_2) (0.8 0.8 0.8))
            (`GameplayStatics.SpawnSoundAtLocation` "/LPSPSample/LPSPSample/Audio/SC_WEP_Impact_Bullet.SC_WEP_Impact_Bullet" (`.ImpactPoint` (`GameplayStatics.BreakHitResult` (`self.HitResult`))) (struct) 1.0 1.0 0.0 null null)
            (message `/LPSPSample/LPSPSample/Core/BPI_LPSP_Damageable.On Receive Damage Point` (`.HitActor` (`GameplayStatics.BreakHitResult` (`self.HitResult`))))))))))

(fn `Get Ammunition Current`
  (returns (ReturnValue :type Integer))
  (return (`self.AmmunitionCurrent`)))

(fn `Get Ammunition Total`
  (returns (ReturnValue :type Integer))
  (return (`self.AmmunitionMax`)))

(fn `Get Rate Of Fire`
  (returns (ReturnValue :type "Float (double-precision)"))
  (return (`self.RateOfFire`)))

(fn `Get Texture Weapon Body`
  (returns (ReturnValue :type "Texture Object Reference"))
  (return (`self.TextureWeaponBody`)))

(fn `Get Texture Weapon Ironsights`
  (returns (ReturnValue :type "Texture Object Reference"))
  (return (`self.TextureWeaponIronsights`)))

(fn `Get Texture Weapon Magazine`
  (returns (ReturnValue :type "Texture Object Reference"))
  (return (`self.TextureWeaponMagazine`)))

(fn `Is Automatic`
  (returns (ReturnValue :type Boolean))
  (return (`self.bAutomatic`)))

(fn `Is Empty`
  (returns (ReturnValue :type Boolean))
  (return (== (`self.AmmunitionCurrent`) 0)))

(fn `UserConstructionScript`)