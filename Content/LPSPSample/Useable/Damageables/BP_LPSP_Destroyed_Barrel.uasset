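; BP_LPSP_Destroyed_Barrel is a damageable's destroyed-barrel actor that pushes nearby objects with a blast impulse when it spawns.
; After calling the parent BeginPlay and a brief delay, it sphere-overlaps mesh components of several object types around its location.
; Each found component receives a linear-falloff radial impulse from the barrel's origin.
; Search radius, impulse radius and strength are randomized within ranges.
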(event `self.ReceiveBeginPlay`
  ;[1 1 1] Begin Play
  (`parent.ReceiveBeginPlay`)
  (`KismetSystemLibrary.Delay` 0.1)
  (bind _outcomponents (`KismetSystemLibrary.SphereOverlapComponents` (`self.K2_GetActorLocation`) (`KismetMathLibrary.RandomFloatInRange` 275.0 325.0) (`|MakeArray` "ObjectTypeQuery1" "ObjectTypeQuery2" "ObjectTypeQuery4" "ObjectTypeQuery8" :!type "EObjectTypeQuery Enum") "/Script/Engine.MeshComponent"))
  (for _array_element _outcomponents
    (`PrimitiveComponent.AddRadialImpulse` _array_element (`self.K2_GetActorLocation`) (`KismetMathLibrary.RandomFloatInRange` 275.0 325.0) (`KismetMathLibrary.RandomFloatInRange` 180000.0 259200.0) "RIF_Linear" false)))

(fn `UserConstructionScript`
  (`parent.UserConstructionScript`))